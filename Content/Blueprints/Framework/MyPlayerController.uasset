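; Player controller that owns the game's HUD, enemy-selection and finish-game screens.
; On BeginPlay it creates all three widgets and adds them to the viewport, keeping the selection and finish screens collapsed.
; Two display events show or hide those screens, switching between UI-only input with cursor and game-only input without it.
; Hiding the finish screen also calls the restart event on the MyGame game mode.
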(event Custom|EventFinishGameDisplay
  (params (Display :type Boolean))
  (bind _finishgamedisplay (Variables|Default|GetFinishGameDisplay))
  (if Display
    (Widget|SetVisibility _finishgamedisplay "Visible")
    (Input|SetInputModeUIOnly (Game|GetPlayerController 0) _finishgamedisplay "DoNotLock" false)
    (Variables|Default|SetbShowMouseCursor true)
    (else
      (Widget|SetVisibility (Variables|Default|GetFinishGameDisplay) "Collapsed")
      (Input|SetInputModeGameOnly (Game|GetPlayerController 0) false)
      (Variables|Default|SetbShowMouseCursor false)
      (bind _asmy_game (Utilities|Casting|CastToMyGame (Game|GetGameMode)))
      (Default|EventRestartGame _asmy_game))))

(event Custom|EventSelectEnemyDisplay
  (params (Display :type Boolean))
  (bind _selectenemydisplay (Variables|Default|GetSelectEnemyDisplay))
  (if Display
    (Widget|SetVisibility _selectenemydisplay "Visible")
    (Input|SetInputModeUIOnly (Game|GetPlayerController 0) _selectenemydisplay "DoNotLock" false)
    (Variables|Default|SetbShowMouseCursor true)
    (else
      (Widget|SetVisibility (Variables|Default|GetSelectEnemyDisplay) "Collapsed")
      (Input|SetInputModeGameOnly (Game|GetPlayerController 0) false)
      (Variables|Default|SetbShowMouseCursor false))))

(event EventBeginPlay
  (bind _returnvalue (UserInterface|CreateWidget "/Game/Blueprints/UI/BPW_HeadupDisplay.BPW_HeadupDisplay_C"))
  (bind _output_get (Variables|Default|SetheadupDisplay _returnvalue))
  (UserInterface|Viewport|AddtoViewport _output_get 0)
  (bind _returnvalue_2 (UserInterface|CreateWidget "/Game/Blueprints/UI/BPW_SelectEnemyDisplay.BPW_SelectEnemyDisplay_C"))
  (bind _output_get_2 (Variables|Default|SetSelectEnemyDisplay _returnvalue_2))
  (Widget|SetVisibility _output_get_2 "Collapsed")
  (UserInterface|Viewport|AddtoViewport _output_get_2 0)
  (bind _returnvalue_3 (UserInterface|CreateWidget "/Game/Blueprints/UI/BPW_FinishGameDIsplay.BPW_FinishGameDIsplay_C"))
  (bind _output_get_3 (Variables|Default|SetFinishGameDisplay _returnvalue_3))
  (Widget|SetVisibility _output_get_3 "Collapsed")
  (UserInterface|Viewport|AddtoViewport _output_get_3 0))

(event EventTick
  (params (DeltaSeconds :type Float%20%28single-precision%29)))

(fn ConstructionScript)