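; BP_Bullet is a projectile actor that registers a hit on its designated enemy bot.
; Mesh overlaps collect unique BP_Bot_Multiplay actors, rescanned through a next-tick loop for the target EnemyActor.
; A match triggers a short delay, DestroyActor, then SR_Attack, which forwards to Attack.
; Unless the enemy has a barrier, Attack flags it as attacked and updates MyActor's cooldown and kill arrays at EnemyIdx.
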(event OnComponentBeginOverlap(StaticMesh)
  (params (OverlappedComponent :type Primitive%20Component%20Object%20Reference) (OtherActor :type Actor%20Object%20Reference) (OtherComp :type Primitive%20Component%20Object%20Reference) (OtherBodyIndex :type Integer) (bFromSweep :type Boolean) (SweepResult :type Hit%20Result%20Structure%20%28by%20ref%29))
  (bind _asbp_bot_multiplay (Utilities|Casting|CastToBP_Bot_Multiplay OtherActor))
  (if (not (Utilities|Array|ContainsItem (Variables|Default|Gettemp) _asbp_bot_multiplay))
    (Utilities|Array|Add (Variables|Default|Gettemp) _asbp_bot_multiplay)
    (for _array_element (Variables|Default|Gettemp) :!label _label
      (if (== _array_element (Variables|Default|GetEnemyActor))
        (Utilities|FlowControl|Delay 0.2)
        (Actor|DestroyActor)
        (CallFunction|SRAttack)))
    (Utilities|FlowControl|DelayUntilNextTick)
    (goto _label)))

(event Custom|Attack
  (bind _myactor (Variables|Default|GetMyActor))
  (if (not (Variables|/Game/Blueprints/Character/BP_Bot_Multiplay.BP_Bot_Multiplay_C|GetIsBarrier (Variables|Default|GetEnemyActor)))
    (Variables|/Game/Blueprints/Character/BP_Bot_Multiplay.BP_Bot_Multiplay_C|SetIsAttacked (Variables|Default|GetEnemyActor) true)
    (Utilities|Array|SetArrayElem (Variables|/Game/Blueprints/Character/BP_Bot_Multiplay.BP_Bot_Multiplay_C|GetEnemyCoolTime _myactor) (Variables|Default|GetEnemyIdx) (Variables|/Game/Blueprints/Character/BP_Bot_Multiplay.BP_Bot_Multiplay_C|GetCEnemyCoolTime _myactor))
    (Utilities|Array|SetArrayElem (Variables|/Game/Blueprints/Character/BP_Bot_Multiplay.BP_Bot_Multiplay_C|GetKillEnemyBotIdx (Variables|Default|GetMyActor)) (Variables|Default|GetEnemyIdx) true)))

(event Custom|SR_Attack
  (CallFunction|Attack))

(event EventBeginPlay)

(event Collision|EventActorBeginOverlap
  (params (OtherActor :type Actor%20Object%20Reference)))

(event EventTick
  (params (DeltaSeconds :type Float%20%28single-precision%29)))

(fn ConstructionScript)

(fn Check)